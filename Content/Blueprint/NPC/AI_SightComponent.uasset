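; AI sight component that lets an NPC detect whether the player is in front of it.
; Trace sphere-traces from a given start point along the owner's forward vector, using configurable range, radius, object types and ignored actors.
; It sets a hit flag only when the first blocking hit is a PlayerCharacter, which GetHitPlayer exposes.
; It does not tick, so detection updates only when Trace is called.
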(event EventBeginPlay
  (Variables|Private|SetOwner (Components|GetOwner)))

(fn Trace
  (params (Start%20Location :type Vector))
  (bind _outhit (Collision|SphereTraceForObjects Start%20Location (+ (* (Transformation|GetActorForwardVector (Variables|Private|GetOwner)) (Variables|TraceSettings|GetTrace%20Multipler)) Start%20Location) (Variables|TraceSettings|GetTrace%20Radius) (Variables|TraceSettings|GetObject%20Types%20To%20Trace) (Variables|TraceSettings|GetTrace%20Complex) (Variables|TraceSettings|GetActors%20Ignore) (Variables|DebugSettings|GetDraw%20Debug%20Type) true "(R=1.000000,G=0.000000,B=0.000000,A=1.000000)" "(R=0.000000,G=1.000000,B=0.000000,A=1.000000)" 0.0))
  (if (.bBlockingHit (Collision|BreakHitResult _outhit))
    (Utilities|Casting|CastToPlayerCharacter (.HitActor (Collision|BreakHitResult _outhit))
      (:then
        (Variables|Private|SetHit%20Player? true))
      (:CastFailed
        (Variables|Private|SetHit%20Player? false)))
    (else
      (Variables|Private|SetHit%20Player? false))))

(fn GetHitPlayer
  (return (Variables|Private|GetHit%20Player?)))