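; BP_TurretShield is a turret shield actor that shows a ripple-style impact effect when hit by projectiles.
; On BeginPlay it creates a dynamic material instance from the Cube mesh's material.
; When the Box collision is hit by a SplitSecondProjectile, it writes the impact point to the material.
; A timeline then animates the impact radius parameter, scaled by a size multiplier.
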(event OnComponentHit(Box)
  (params (HitComponent :type Primitive%20Component%20Object%20Reference) (OtherActor :type Actor%20Object%20Reference) (OtherComp :type Primitive%20Component%20Object%20Reference) (NormalImpulse :type Vector :default "0, 0, 0") (Hit :type Hit%20Result%20Structure%20%28by%20ref%29))
  ;[1 1 1] Bullet Impact Effect
  (Utilities|Casting|CastToSplitSecondProjectile OtherActor)
  (Rendering|Material|SetVectorParameterValue (Variables|Private|GetShield%20Mat) "Impact Pos" (Math|Conversions|ToLinearColor(Vector) (.impactpoint Hit)) :!class /Script/Engine.MaterialInstanceDynamic)
  (bind _radius_track (Timeline|Impact%20Animation PlayFromStart)
    (:Update
      (Rendering|Material|SetScalarParameterValue (Variables|Private|GetShield%20Mat) "Impact Radius" (* _radius_track (Variables|Settings|GetImpact%20Size%20Multipler)) :!class /Script/Engine.MaterialInstanceDynamic))))

(event EventBeginPlay
  ;[1 1 1] Create a dynamic Material to edit shield mat
  (bind _returnvalue (Rendering|Material|CreateDynamicMaterialInstance (Variables|Default|GetCube) 0 0 "None" :!class /Script/Engine.PrimitiveComponent))
  (Variables|Private|SetShield%20Mat _returnvalue))

(fn ConstructionScript)