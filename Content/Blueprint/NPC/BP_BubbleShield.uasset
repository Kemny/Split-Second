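; Bubble shield actor for NPCs that fades in and out and shows a ripple where projectiles strike it.
; A dynamic material receives timeline-driven opacity and, on SplitSecondProjectile hits while active, the impact point and animated radius.
; ActivateShield makes the sphere block pawns and a custom channel once faded in; DeactivateShield fades out, then destroys the actor.
; KnockbackPlayer is an empty stub.
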(event OnComponentHit(Sphere)
  (params (HitComponent :type Primitive%20Component%20Object%20Reference) (OtherActor :type Actor%20Object%20Reference) (OtherComp :type Primitive%20Component%20Object%20Reference) (NormalImpulse :type Vector :default "0, 0, 0") (Hit :type Hit%20Result%20Structure%20%28by%20ref%29))
  ;[1 1 1] Bullet Impact Effect
  (if (Variables|Default|GetIs%20Shield%20Up?)
    (Utilities|Casting|CastToSplitSecondProjectile OtherActor)
    (Rendering|Material|SetVectorParameterValue (Variables|Default|GetShield%20Mat) "Impact Pos" (Math|Conversions|ToLinearColor(Vector) (.impactpoint Hit)) :!class /Script/Engine.MaterialInstanceDynamic)
    (bind _radius_track (Timeline|Timeline_0 PlayFromStart)
      (:Update
        (Rendering|Material|SetScalarParameterValue (Variables|Default|GetShield%20Mat) "Impact Radius" (* _radius_track (Variables|Default|GetImpact%20Size%20Multipler)) :!class /Script/Engine.MaterialInstanceDynamic)))))

(event EventBeginPlay
  ;[1 1 1] Create a dynamic Material to edit shield mat
  (bind _returnvalue (Rendering|Material|CreateDynamicMaterialInstance (Variables|Default|GetShield) 0 0 "None" :!class /Script/Engine.PrimitiveComponent))
  (Variables|Default|SetShield%20Mat _returnvalue))

(event EventActivateShield
  ;[1 1 1] Fade in Shield
  (Variables|Default|SetIs%20Shield%20Up? true)
  (bind _fade_track (Timeline|Fade%20in%20Shield Play)
    (:Update
      (Rendering|Material|SetScalarParameterValue (Variables|Default|GetShield%20Mat) "Opacity" _fade_track :!class /Script/Engine.MaterialInstanceDynamic))
    (:Finished
      (Collision|SetCollisionResponsetoChannel (Variables|Default|GetSphere) "ECC_GameTraceChannel2" "ECR_Block")
      (Collision|SetCollisionResponsetoChannel (Variables|Default|GetSphere) "ECC_Pawn" "ECR_Block"))))

(event EventDeactivateShield
  ;[1 1 1] Fade out Shield
  (Variables|Default|SetIs%20Shield%20Up? false)
  (bind _fade_track (Timeline|Fade%20Out%20Shield Play)
    (:Update
      (Rendering|Material|SetScalarParameterValue (Variables|Default|GetShield%20Mat) "Opacity" _fade_track :!class /Script/Engine.MaterialInstanceDynamic))
    (:Finished
      (Actor|DestroyActor))))

(fn ConstructionScript)

(fn KnockbackPlayer)