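; BP_FireTrap is a world trap whose fire toggles on and off at a fixed interval and hurts players who touch it.
; A looping timer started at BeginPlay alternates the Niagara fire effect and the damage flag together.
; The box overlap applies damage to a PlayerCharacter only if the fire is on at the moment of entry, so standing inside as it ignites deals nothing.
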(event OnComponentBeginOverlap(Box)
  (params (OverlappedComponent :type Primitive%20Component%20Object%20Reference) (OtherActor :type Actor%20Object%20Reference) (OtherComp :type Primitive%20Component%20Object%20Reference) (OtherBodyIndex :type Integer) (bFromSweep :type Boolean) (SweepResult :type Hit%20Result%20Structure%20%28by%20ref%29))
  (bind _asplayer_character (Utilities|Casting|CastToPlayerCharacter OtherActor))
  (if (Variables|Default|GetCan%20Damage?)
    (Game|Damage|ApplyDamage _asplayer_character (Variables|Default|GetDamage) 0 self)))

(event Custom|Turn%20On%20Fire
  (if (not (Variables|Default|GetFire%20up?))
    (Components|Activation|Activate (Variables|Default|GetNiagara) false)
    (Variables|Default|SetFire%20up? true)
    (Variables|Default|SetCan%20Damage? true)
    (else
      (Components|Activation|Deactivate (Variables|Default|GetNiagara))
      (Variables|Default|SetFire%20up? false)
      (Variables|Default|SetCan%20Damage? false))))

(event EventBeginPlay
  (Components|Activation|Deactivate (Variables|Default|GetNiagara))
  (Utilities|Time|SetTimerbyEvent (delegate Custom|Turn%20On%20Fire) (Variables|Default|GetTrapInterval) true))

(fn ConstructionScript)