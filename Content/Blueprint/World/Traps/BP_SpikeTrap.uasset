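; BP_SpikeTrap is a world trap that periodically raises and removes a spike.
; A looping timer started on BeginPlay alternates between spawning a half-scale BP_Spike just above the trap and destroying it after a short delay.
; A flag tracks the spike state, and each spawned spike receives a reference to its trap.
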(event Custom|Spawn%20Spike
  (bind _returnvalue (Transformation|GetActorLocation))
  (if (not (Variables|Default|GetIs%20Spike%20Up?))
    (bind _returnvalue_2 (Game|SpawnActorfromClass "/Game/Blueprint/World/Traps/BP_Spike.BP_Spike_C" (Math|Transform|MakeTransform (Math|Vector|MakeVector (.x _returnvalue) (.y _returnvalue) (+ (.z _returnvalue) 1e+02)) "0, 0, 0" "0.500000,0.500000,0.500000") "Undefined" 0 self 0))
    (Variables|Default|SetCurrent%20Spike _returnvalue_2)
    (Variables|Default|SetIs%20Spike%20Up? true)
    (else
      (Utilities|FlowControl|Delay 1.0)
      (Actor|DestroyActor (Variables|Default|GetCurrent%20Spike))
      (Variables|Default|SetIs%20Spike%20Up? false))))

(event EventBeginPlay
  (Utilities|Time|SetTimerbyEvent (delegate Custom|Spawn%20Spike) (Variables|Default|GetTrapInterval) true))

(fn ConstructionScript)